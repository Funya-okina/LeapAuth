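; Actor that records Leap Motion hand-tracking data and shows the palm position as debug text.
; It starts tracking in desktop mode and switches to VR mode when another actor overlaps it.
; While either hand is visible, each tracking frame appends the first hand's finger-extended flags and palm position to HandData, then draws the new position.
; HandData is never cleared here, so it grows with every tracked frame.
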(event OnLeapTrackingData(Leap)
  (params (Frame :type Leap%20Frame%20Data%20Structure%20%28by%20ref%29))
  (bind (_numberofhandsvisible _framerate _hands _frameid _lefthandvisible _righthandvisible) (Utilities|Struct|BreakLeapFrameData Frame))
  (bind _handdata (Variables|Default|GetHandData))
  (bind _output (Utilities|Array|Get(acopy) _hands))
  (bind (_arm _confidence _digits _flags _grabangle _grabstrength _handtype _index _middle _palm _pinchdistance _pinchstrength _pinky _ring _thumb) (Utilities|Struct|BreakLeapHandData _output))
  (if (or _lefthandvisible _righthandvisible)
    (bind _returnvalue (Utilities|Array|Add _handdata (Utilities|Struct|MakeHandData (Utilities|Array|MakeArray (.IsExtended (Utilities|Struct|BreakLeapDigitData _thumb)) (.IsExtended (Utilities|Struct|BreakLeapDigitData _index)) (.IsExtended (Utilities|Struct|BreakLeapDigitData _middle)) (.IsExtended (Utilities|Struct|BreakLeapDigitData _ring)) (.IsExtended (Utilities|Struct|BreakLeapDigitData _pinky))) (.Position (Utilities|Struct|BreakLeapPalmData _palm)))))
    (Rendering|Debug|DrawDebugString "0, 0, 0" (Utilities|String|BuildString(Vector) "" "" (.HandPosition (Utilities|Struct|BreakHandData (Utilities|Array|Get(acopy) _handdata _returnvalue)))) 0 "(R=1.000000,G=1.000000,B=1.000000,A=1.000000)")))

(event EventBeginPlay
  (Class|LeapBlueprintFunctionLibrary|SetLeapMode "LEAP_MODE_DESKTOP" "LEAP_NORMAL"))

(event Collision|EventActorBeginOverlap
  (params (OtherActor :type Actor%20Object%20Reference))
  (Class|LeapBlueprintFunctionLibrary|SetLeapMode "LEAP_MODE_VR" "LEAP_NORMAL"))

(event EventTick
  (params (DeltaSeconds :type Float%20%28single-precision%29)))

(fn ConstructionScript)